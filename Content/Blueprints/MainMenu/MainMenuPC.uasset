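; MainMenuPC is the main menu player controller that manages which menu screen is on the viewport.
; On BeginPlay it sets UI-only input without mouse lock, shows the cursor and opens the main menu.
; Separate events for the main, server and login menus each remove all widgets, then create and add their own widget.
; The login menu event is marked out of order and is not called here.
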(event Custom|ShowServerMenu
  (Viewport|RemoveAllWidgets)
  (bind _returnvalue (UserInterface|CreateWidget "/Game/UI/MainMenu/ServerMenuWB.ServerMenuWB_C"))
  (UserInterface|Viewport|AddtoViewport _returnvalue 0))

(event Custom|ShowLoginMenu
  (Viewport|RemoveAllWidgets)
  (bind _returnvalue (UserInterface|CreateWidget "/Game/UI/MainMenu/LoginMenuWB.LoginMenuWB_C"))
  (UserInterface|Viewport|AddtoViewport _returnvalue 0))

(event Custom|ShowMainMenu
  (Viewport|RemoveAllWidgets)
  (bind _returnvalue (UserInterface|CreateWidget "/Game/UI/MainMenu/MainMenuWB.MainMenuWB_C"))
  (UserInterface|Viewport|AddtoViewport _returnvalue 0))

(event EventBeginPlay
  (Input|SetInputModeUIOnly self 0 "DoNotLock")
  (Variables|Default|SetbShowMouseCursor true)
  (CallFunction|ShowMainMenu))

(fn ConstructionScript)