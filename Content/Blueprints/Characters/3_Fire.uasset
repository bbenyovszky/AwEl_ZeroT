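; Fire character child Blueprint with a short-range continuous beam weapon, fired while left mouse is held.
; On authority, Tick drains stamina and applies frame-scaled point damage, stopping when stamina runs out.
; A camera trace picks the aim point, then a fixed-length trace from the weapon's AmmoSocket finds the hit and sets the beam target.
; Client start/stop events manage muzzle-attached laser particles and sound; death also stops firing.
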(event Custom|StartShooting
  (Variables|Default|SetShooting true)
  (CallFunction|StartShootingClient))

(event Custom|StopShooting
  (Variables|Default|SetShooting false)
  (CallFunction|StopShootingClient))

(event Custom|Tick_Shooting
  (bind _followcamera (Variables|Default|GetFollowCamera))
  (bind _weapon (Variables|Default|GetWeapon))
  (bind _returnvalue (Transformation|GetWorldLocation _followcamera))
  (bind _skeletalmesh (Variables|/Game/Blueprints/FPWeapon/SK_FPGun.SK_FPGun_C|GetSkeletalMesh _weapon))
  (bind _returnvalue_2 (Transformation|GetSocketLocation _skeletalmesh "AmmoSocket"))
  (if (Variables|Default|GetShooting)
    (if (> (Variables|Default|GetCurrentStamina) 0.0)
      (CallFunction|SubtractStamina (* (Utilities|Time|GetWorldDeltaSeconds) (Variables|Default|GetShootingStaminaRate)))
      (bind _outhit (Collision|LineTraceByChannel _returnvalue (+ _returnvalue (* (Math|Vector|GetForwardVector (Transformation|GetWorldRotation _followcamera)) 6000)) "TraceTypeQuery2" false 0 "None"))
      (bind _outhit_2 (Collision|LineTraceByChannel _returnvalue_2 (+ (Math|Vector|ClampVectorSize (- (Math|Vector|SelectVector (.location _outhit) (.traceend _outhit) (.bblockinghit _outhit)) _returnvalue_2) 3e+02 3e+02) _returnvalue_2) "TraceTypeQuery2" true (Utilities|Array|MakeArray _weapon) "None"))
      (Game|Damage|ApplyPointDamage (.HitActor (Collision|BreakHitResult _outhit_2)) (* (Utilities|Time|GetWorldDeltaSeconds) (Variables|Default|GetFireRate)) (.TraceStart (Collision|BreakHitResult _outhit_2)) _outhit_2 (Pawn|GetController))
      (CallFunction|ShootEffect (.TraceStart (Collision|BreakHitResult _outhit_2)) (Math|Vector|SelectVector (.Location (Collision|BreakHitResult _outhit_2)) (.TraceEnd (Collision|BreakHitResult _outhit_2)) (.bBlockingHit (Collision|BreakHitResult _outhit_2))))
      (else
        (CallFunction|StopShooting)))))

(event Custom|StartShooting_Client
  (bind _returnvalue (Utilities|Name|MakeLiteralName "Muzzle"))
  (bind _weapon (Variables|Default|GetWeapon))
  (bind _skeletalmesh (Variables|/Game/Blueprints/FPWeapon/SK_FPGun.SK_FPGun_C|GetSkeletalMesh _weapon))
  (bind _returnvalue_2 (Effects|SpawnEmitterAttached "/Game/Effects/1_Light/P_Beam_Laser.P_Beam_Laser" _skeletalmesh _returnvalue "0.000000, 0, 0" "0, 0, 0" "SnapToTargetIncludingScale" false))
  (Variables|Default|SetLaserEffect _returnvalue_2)
  (bind _returnvalue_3 (Audio|SpawnSoundAttached "/Game/StarterContent/Audio/Light01.Light01" _skeletalmesh _returnvalue "0, 0, 0" "0, 0, 0" "SnapToTarget" true 5.0 1.0 0.0))
  (Variables|Default|SetLaserSoundEffect _returnvalue_3))

(event Custom|StopShooting_Client
  (bind _lasersoundeffect (Variables|Default|GetLaserSoundEffect))
  (bind _lasereffect (Variables|Default|GetLaserEffect))
  (Utilities|FlowControl|Sequence
    (:then_0
      (Utilities|IsValid _lasereffect ; Not valid on Dedicated server
        (:Is%20Valid
          (Components|DestroyComponent _lasereffect))))
    (:then_1
      (Utilities|IsValid _lasersoundeffect
        (:Is%20Valid
          (Audio|Components|Audio|Stop _lasersoundeffect)
          (Components|DestroyComponent _lasersoundeffect))))))

(event Custom|ShootEffect
  (params (From :type Vector) (To :type Vector))
  (bind _lasereffect (Variables|Default|GetLaserEffect))
  (Utilities|IsValid _lasereffect ; Not: Dedicated server
    (:Is%20Valid
      (Class|ParticleSystemComponent|SetBeamTargetPoint _lasereffect 0 To))))

(event EventTick
  (params (DeltaSeconds :type Float%20%28single-precision%29))
  (|CallParentFunction DeltaSeconds)
  (Networking|SwitchHasAuthority
    (:Authority
      (Utilities|FlowControl|Sequence
        (:then_0
          (CallFunction|TickShooting))))))

(event EventDeath
  (|CallParentFunction)
  (CallFunction|StopShooting))

(event Input|MouseEvents|LeftMouseButton
  (params (Key :type Key%20Structure :default "AnyKey"))
  (:Pressed
    (CallFunction|StartShooting))
  (:Released
    (CallFunction|StopShooting)))

(fn ConstructionScript
  (|CallParentFunction))